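; Interactable swinging door that the player opens and closes with E while overlapping it.
; BeginPlay caches the placed rotation as closed and adds 90 degrees of yaw for open, so it works at any starting orientation.
; Actor overlap events toggle input for player 0 without checking which actor overlapped.
; The OpenDoor timeline plays or reverses to lerp actor rotation, blocking interaction until it finishes.
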(event `self.ReceiveBeginPlay`
  ;[0.7943 0.7296 1] Vid start: uppdatera dörrens rotations variabler (basically nollställa dörrens rotation i scenen oavsett hur den är roterad vid start)
  (bind _output_get (set `self.Start rot` (`self.K2_GetActorRotation`)))
  (set `self.End rot` (`KismetMathLibrary.MakeRotator` (.roll _output_get) (.pitch _output_get) (+ (.yaw _output_get) 90.0))))

(event `self.ReceiveActorBeginOverlap`
  (params (OtherActor :type "Actor Object Reference"))
  ;[1 0.8917 0.5948] När spelaren står inom range av den här dörrens box collision: Tillåt spelaren att interagera.
  (`self.EnableInput` (`GameplayStatics.GetPlayerController` 0)))

(event `Key|E`
  (params (Key :type "Key Structure"))
  ;[0.6445 1 0.8114] När spelaren trycker på E
  (:`Pressed`
    ;[1 1 1] Kan spelaren interagera? (om dörren redan öppnas kan man inte interagere)
    (if (`self.CanInteract`)
      ;[1 1 1] Är dörren öppen eller stängd?
      (if (`self.IsOpen`)
        ;[0.2393 1 0.9801] Öppna/stäng dörren efter en timeline (den gula noden)
        (set `self.IsOpen` false)
        (bind (_direction _opening) (`Timeline|OpenDoor` :!via `Reverse` :!label _label)
          (:`Update`
            ;[1 1 1] Sätt en ny rotation efter lerp värdena. Spelaren kan inte interagera med dörren under den här tiden.
            (`self.K2_SetActorRotation` (`KismetMathLibrary.RLerp` (`self.Start rot`) (`self.End rot`) _opening))
            (set `self.CanInteract` false))
          (:`Finished`
            ;[1 1 1] När animationen är klar kan spelaren interagera igen
            (set `self.CanInteract` true)))
        (else
          (set `self.IsOpen` true)
          (goto _label))))))

(event `self.ReceiveActorEndOverlap`
  (params (OtherActor :type "Actor Object Reference"))
  ;[0.4499 0.8278 1] När spelaren lämnar box collision: låt inte spelaren interagera.
  (`self.DisableInput` (`GameplayStatics.GetPlayerController` 0)))

(fn `UserConstructionScript`)