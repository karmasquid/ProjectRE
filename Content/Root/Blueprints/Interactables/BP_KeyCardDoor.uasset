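; A key card door that slides vertically when a player holding a key presses E nearby.
; Overlap begin and end toggle the actor's input for the first player controller.
; The E press casts the overlapping actor to FirstPersonCharacter and checks that its Key count is above zero, without decrementing it.
; A timeline then offsets the door's Z from the location cached at BeginPlay, with no closing logic.
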(event `self.ReceiveBeginPlay`
  (set `self.Location` (`self.K2_GetActorLocation`)))

(event `self.ReceiveActorBeginOverlap`
  (params (OtherActor :type "Actor Object Reference"))
  (`self.EnableInput` (`GameplayStatics.GetPlayerController` 0)))

(event `Key|E`
  (params (Key :type "Key Structure"))
  (bind (_location_x _location_y _location_z) (`KismetMathLibrary.BreakVector` (`self.Location`)))
  (:`Pressed`
    (bind _asfirst_person_character (cast `/Game/Core/Player/FirstPersonCharacter` (stale `self.ReceiveActorBeginOverlap` OtherActor)))
    (if (> (`/Game/Core/Player/FirstPersonCharacter.Key` _asfirst_person_character) 0)
      (bind (_direction _newtrack_0 _newtrack_1) (`Timeline|Timeline_0`)
        (:`Update`
          (`self.K2_SetActorLocation` (`KismetMathLibrary.MakeVector` _location_x _location_y (+ _newtrack_0 _location_z))))))))

(event `self.ReceiveActorEndOverlap`
  (params (OtherActor :type "Actor Object Reference"))
  (`self.DisableInput` (`GameplayStatics.GetPlayerController` 0)))

(fn `UserConstructionScript`)