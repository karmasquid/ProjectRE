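; BP_LockedDoor is an interactable door that shows a locked-door message when E is pressed while input is enabled.
; Actor overlap begin and end enable and disable its input for player controller 0, without checking which actor overlaps.
; Each press adds a new Widget_LockedDoor to the viewport, waits briefly, then removes top-level widgets of that class.
; It contains no unlock or opening logic.
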(event `self.ReceiveActorBeginOverlap`
  (params (OtherActor :type "Actor Object Reference"))
  (`self.EnableInput` (`GameplayStatics.GetPlayerController` 0)))

(event `Key|E`
  (params (Key :type "Key Structure"))
  (:`Pressed`
    (bind _returnvalue (`|CreateWidget` "/Game/Root/Blueprints/Pickups/Widget_LockedDoor.Widget_LockedDoor_C"))
    (`UserWidget.AddToViewport` _returnvalue 0)
    (`KismetSystemLibrary.Delay` 4.0)
    (bind _foundwidgets (`WidgetBlueprintLibrary.GetAllWidgetsOfClass` (`GameplayStatics.GetObjectClass` _returnvalue)))
    (`Widget.RemoveFromParent` _foundwidgets)))

(event `self.ReceiveActorEndOverlap`
  (params (OtherActor :type "Actor Object Reference"))
  (`self.DisableInput` (`GameplayStatics.GetPlayerController` 0)))

(fn `UserConstructionScript`)