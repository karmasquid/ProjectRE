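; BP_Elevator is an interactable elevator that moves its Floor component between two positions when the player presses E.
; Actor overlap enables and disables player input, so the key works only while something overlaps the elevator.
; Each press flips Floor01 and plays or reverses a timeline that lerps the relative location from Position1 to Position2.
; CanControll blocks further presses during movement and is restored when the timeline finishes.
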(event `self.ReceiveActorBeginOverlap`
  (params (OtherActor :type "Actor Object Reference"))
  (`self.EnableInput` (`GameplayStatics.GetPlayerController` 0)))

(event `self.ReceiveActorEndOverlap`
  (params (OtherActor :type "Actor Object Reference"))
  (`self.DisableInput` (`GameplayStatics.GetPlayerController` 0)))

(event `Key|E`
  (params (Key :type "Key Structure"))
  (:`Pressed`
    (if (`self.CanControll`)
      ;[1 1 1] Am I on Floor 1?
      (if (`self.Floor01`)
        (set `self.Floor01` false)
        ;[1 0.2837 0.1437] En hiss funkar likadant fast har vectorer (gula trådar) istället för rotation (gråa trådar). Sen så används SetRelativeLocation som nod istället för SetActorRotation
        (bind (_direction _newtrack_1) (`Timeline|Timeline_0` :!label _label)
          (:`Update`
            (`SceneComponent.K2_SetRelativeLocation` (`self.Floor`) (`KismetMathLibrary.VLerp` (`self.Position1`) (`self.Position2`) _newtrack_1) false false)
            (set `self.CanControll` false))
          (:`Finished`
            (set `self.CanControll` true)))
        (else
          (set `self.Floor01` true)
          (goto _label :!via `Reverse`))))))

(fn `UserConstructionScript`)