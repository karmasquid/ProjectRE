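; BP_OneDirectionLabDoor is an interactable sliding door that opens on a key press and closes by itself.
; Actor overlap enables input from player 0, and ending the overlap disables it.
; Pressing E while closed plays the Moving timeline, lerping the actor from its starting location to Pos2.
; After a short delay CloseDoor reverses the timeline, with IsOpen guarding against retriggering.
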(event `self.ReceiveBeginPlay`
  (set `self.Pos1` (`self.K2_GetActorLocation`)))

(event `self.ReceiveActorBeginOverlap`
  (params (OtherActor :type "Actor Object Reference"))
  (`self.EnableInput` (`GameplayStatics.GetPlayerController` 0)))

(event `Key|E`
  (params (Key :type "Key Structure"))
  (:`Pressed`
    (if (not (`self.IsOpen`))
      (set `self.IsOpen` true)
      (bind (_direction _newtrack_0) (`Timeline|Moving` :!label _label)
        (:`Update`
          (`self.K2_SetActorRelativeLocation` (`KismetMathLibrary.VLerp` (`self.Pos1`) (`self.Pos2`) _newtrack_0)))
        (:`Finished`
          (if (`self.IsOpen`)
            (`KismetSystemLibrary.Delay` 3.0)
            (`self.CloseDoor`)
            (set `self.IsOpen` false)))))))

(event `self.ReceiveActorEndOverlap`
  (params (OtherActor :type "Actor Object Reference"))
  (`self.DisableInput` (`GameplayStatics.GetPlayerController` 0)))

(event `CloseDoor`
  (goto _label :!via `ReverseFromEnd`))

(fn `UserConstructionScript`)