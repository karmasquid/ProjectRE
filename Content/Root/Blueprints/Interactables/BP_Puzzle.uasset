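; BP_Puzzle is a rotating puzzle interactable that triggers a linked SpawnPoint's WhenToSpawn once turned enough times.
; Overlap enables player input, and pressing E plays the Rotation timeline, adding yaw to the stored ZRotation until Turn reaches FinalTurn.
; A Delay on the timeline's Update pin postpones advancing the stored yaw by a quarter turn, incrementing Turn and checking for completion.
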(event `self.ReceiveBeginPlay`
  (set `self.Z rotation` (`self.K2_GetActorRotation`)))

(event `self.ReceiveActorBeginOverlap`
  (params (OtherActor :type "Actor Object Reference"))
  (`self.EnableInput` (`GameplayStatics.GetPlayerController` 0)))

(event `Key|E`
  (params (Key :type "Key Structure"))
  (bind _turn (`self.Turn`))
  (bind (_z_rotation_roll _z_rotation_pitch _z_rotation_yaw) (`KismetMathLibrary.BreakRotator` (`self.Z rotation`)))
  (:`Pressed`
    (if (< (`self.Turn`) (`self.FinalTurn`))
      (bind (_direction _rotating) (`Timeline|Rotation` :!via `PlayFromStart`)
        (:`Update`
          (`self.K2_SetActorRotation` (`KismetMathLibrary.MakeRotator` _z_rotation_roll _z_rotation_pitch (+ _rotating _z_rotation_yaw)))
          (`KismetSystemLibrary.Delay` 5.0)
          (set `self.Z rotation` (`KismetMathLibrary.MakeRotator` _z_rotation_roll _z_rotation_pitch (+ _z_rotation_yaw 90.0)))
          (`/Engine/EditorBlueprintResources/StandardMacros.IncrementInt` _turn
            (:`  `
              (if (== _turn (`self.FinalTurn`))
                (`/Game/Root/Blueprints/BP_KeySpawnPoint.WhenToSpawn` (`self.SpawnPoint`))))))))))

(event `self.ReceiveActorEndOverlap`
  (params (OtherActor :type "Actor Object Reference"))
  (`self.DisableInput` (`GameplayStatics.GetPlayerController` 0)))

(fn `UserConstructionScript`)