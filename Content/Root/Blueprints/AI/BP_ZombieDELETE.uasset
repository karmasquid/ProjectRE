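; Zombie AI character, named as slated for deletion, that gives each instance randomized toughness and walk speed.
; On BeginPlay it rolls a small HP value and sets max walk speed to a random value between the movement component's existing speed and a fixed bound.
; Each Takedamage event removes one HP and destroys the actor once HP falls below one.
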(event `self.ReceiveBeginPlay`
  (bind _charactermovement (`self.CharacterMovement`))
  (set `self.HP` (`KismetMathLibrary.RandomFloatInRange` 2.0 5.0))
  (set `CharacterMovementComponent.MaxWalkSpeed` (`KismetMathLibrary.RandomFloatInRange` (`CharacterMovementComponent.MaxWalkSpeed` _charactermovement) 150.0) _charactermovement))

(event `Take damage`
  (bind _hp (`self.HP`))
  (`/Engine/EditorBlueprintResources/StandardMacros.DecrementFloat` _hp
    (:`  `
      (if (< _hp 1.0)
        (`self.K2_DestroyActor`)))))

(fn `UserConstructionScript`)