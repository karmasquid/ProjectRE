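; Code pickup that gives the player the code for the finale and triggers a zombie ambush.
; Any actor overlap enables the pickup's input for player 0, and ending the overlap disables it.
; Pressing E sets HasCode on FinaleTrigger and destroys the pickup, then a second Sequence branch spawns AI zombies running MyBehaviourTree at seven referenced spawn-point actors.
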(event `self.ReceiveActorBeginOverlap`
  (params (OtherActor :type "Actor Object Reference"))
  (`self.EnableInput` (`GameplayStatics.GetPlayerController` 0)))

(event `Key|E`
  (params (Key :type "Key Structure"))
  (:`Pressed`
    (`|ExecutionSequence`
      (:`then_0`
        (set `/Game/Root/Blueprints/BP_FinaleTrigger.HasCode` true (`self.FinaleTrigger`))
        (`self.K2_DestroyActor`))
      (:`then_1`
        (`AIBlueprintHelperLibrary.SpawnAIFromClass` "/Game/Root/Blueprints/AI/BP_ZombieDELETE.BP_ZombieDELETE_C" "/Game/Root/Blueprints/AI/MYBehaviourTree.MyBehaviourTree" (`self.K2_GetActorLocation` (`self.Zombie spawning`)) (struct) false null)
        (`AIBlueprintHelperLibrary.SpawnAIFromClass` "/Game/Root/Blueprints/AI/BP_ZombieDELETE.BP_ZombieDELETE_C" "/Game/Root/Blueprints/AI/MYBehaviourTree.MyBehaviourTree" (`self.K2_GetActorLocation` (`self.Zombie spawning_0`)) (struct) false null)
        (`AIBlueprintHelperLibrary.SpawnAIFromClass` "/Game/Root/Blueprints/AI/BP_ZombieDELETE.BP_ZombieDELETE_C" "/Game/Root/Blueprints/AI/MYBehaviourTree.MyBehaviourTree" (`self.K2_GetActorLocation` (`self.Zombie spawning_1`)) (struct) false null)
        (`AIBlueprintHelperLibrary.SpawnAIFromClass` "/Game/Root/Blueprints/AI/BP_ZombieDELETE.BP_ZombieDELETE_C" "/Game/Root/Blueprints/AI/MYBehaviourTree.MyBehaviourTree" (`self.K2_GetActorLocation` (`self.Zombie spawning_2`)) (struct) false null)
        (`AIBlueprintHelperLibrary.SpawnAIFromClass` "/Game/Root/Blueprints/AI/BP_ZombieDELETE.BP_ZombieDELETE_C" "/Game/Root/Blueprints/AI/MYBehaviourTree.MyBehaviourTree" (`self.K2_GetActorLocation` (`self.Zombie spawning_3`)) (struct) false null)
        (`AIBlueprintHelperLibrary.SpawnAIFromClass` "/Game/Root/Blueprints/AI/BP_ZombieDELETE.BP_ZombieDELETE_C" "/Game/Root/Blueprints/AI/MYBehaviourTree.MyBehaviourTree" (`self.K2_GetActorLocation` (`self.Zombie spawning_4`)) (struct) false null)
        (`AIBlueprintHelperLibrary.SpawnAIFromClass` "/Game/Root/Blueprints/AI/BP_ZombieDELETE.BP_ZombieDELETE_C" "/Game/Root/Blueprints/AI/MYBehaviourTree.MyBehaviourTree" (`self.K2_GetActorLocation` (`self.Zombie spawning_5`)) (struct) false null)))))

(event `self.ReceiveActorEndOverlap`
  (params (OtherActor :type "Actor Object Reference"))
  (`self.DisableInput` (`GameplayStatics.GetPlayerController` 0)))

(fn `UserConstructionScript`)