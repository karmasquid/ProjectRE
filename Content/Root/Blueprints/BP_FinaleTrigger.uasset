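; BP_FinaleTrigger is a trigger actor that spawns the finale's zombie wave when something overlaps it while HasCode is true.
; The overlap event clears HasCode so the wave fires once per set flag, then spawns a BP_Zombie running MyBehaviourTree at each of three referenced spawn point actors.
; The overlap does not filter by actor, and HasCode is not set true anywhere in this graph.
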(event `self.ReceiveActorBeginOverlap`
  (params (OtherActor :type "Actor Object Reference"))
  (if (`self.HasCode`)
    (set `self.HasCode` false)
    (`AIBlueprintHelperLibrary.SpawnAIFromClass` "/Game/Root/Blueprints/AI/BP_Zombie.BP_Zombie_C" "/Game/Root/Blueprints/AI/MYBehaviourTree.MyBehaviourTree" (`self.K2_GetActorLocation` (`self.SpawnPoint1`)) (struct) false null)
    (`AIBlueprintHelperLibrary.SpawnAIFromClass` "/Game/Root/Blueprints/AI/BP_Zombie.BP_Zombie_C" "/Game/Root/Blueprints/AI/MYBehaviourTree.MyBehaviourTree" (`self.K2_GetActorLocation` (`self.SpawnPoint2`)) (struct) false null)
    (`AIBlueprintHelperLibrary.SpawnAIFromClass` "/Game/Root/Blueprints/AI/BP_Zombie.BP_Zombie_C" "/Game/Root/Blueprints/AI/MYBehaviourTree.MyBehaviourTree" (`self.K2_GetActorLocation` (`self.SpawnPoint3`)) (struct) false null)))

(fn `UserConstructionScript`)