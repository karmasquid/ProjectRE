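; Zombie character Blueprint with randomized hit points and walk speed, set on BeginPlay.
; Each Takedamage call removes one HP; below one, it stops the AI controller's brain logic and sets IsDead.
; After a short delay the mesh switches to physics ragdoll and the capsule loses collision.
; After a further delay it broadcasts OnKilled and destroys itself.
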(event `self.ReceiveBeginPlay`
  (bind _charactermovement (`self.CharacterMovement`))
  ;[0.4111 1 0.2042] Setting different HP and movement speed per zombie
  (set `self.HP` (`KismetMathLibrary.RandomFloatInRange` 2.0 7.0))
  (set `CharacterMovementComponent.MaxWalkSpeed` (`KismetMathLibrary.RandomFloatInRange` (`CharacterMovementComponent.MaxWalkSpeed` _charactermovement) 100.0) _charactermovement))

(event `Take damage`
  (bind _hp (`self.HP`))
  (bind _mesh (`self.Mesh`))
  ;[1 0.25 0.25] Damage calculator and death check
  (`/Engine/EditorBlueprintResources/StandardMacros.DecrementFloat` _hp
    (:`  `
      (if (< _hp 1.0)
        (`BrainComponent.StopLogic` (`AIController.BrainComponent` (`AIBlueprintHelperLibrary.GetAIController` self)) "")
        ;[1 1 1] Death and ragdoll
        (set `self.IsDead` true)
        (`KismetSystemLibrary.Delay` 2.9)
        (`PrimitiveComponent.SetCollisionProfileName` _mesh "Ragdoll" true)
        (`PrimitiveComponent.SetSimulatePhysics` _mesh true)
        (`PrimitiveComponent.SetCollisionProfileName` (`self.CapsuleComponent`) "NoCollision" true)
        (`KismetSystemLibrary.Delay` 5.0)
        (`self.OnKilled` self)
        (`self.K2_DestroyActor`)))))

(fn `UserConstructionScript`)