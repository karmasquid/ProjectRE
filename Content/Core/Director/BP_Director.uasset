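; BP_Director is a director Blueprint that tracks the living BP_Zombie actors in the level.
; On BeginPlay it passes every existing zombie to OnZombieSpawned, which adds it to the Zombies array and binds to its OnKilled event.
; OnZombieKilled removes a zombie from the array, and Tick prints the current count on screen as a debug readout.
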(event `self.ReceiveBeginPlay`
  (bind _outactors (`GameplayStatics.GetAllActorsOfClass` "/Game/Root/Zombie/AI_Zombie/BP_Zombie.BP_Zombie_C"))
  (for _array_element _outactors
    (`self.OnZombieSpawned` _array_element)))

(event `self.ReceiveTick`
  (params (DeltaSeconds :type "Float (single-precision)"))
  (`KismetSystemLibrary.PrintString` (`KismetStringLibrary.Concat_StrStr` "Numb zombies" (`KismetStringLibrary.Conv_IntToString` (`KismetArrayLibrary.Array_Length` (`self.Zombies`)))) true true (struct :`G` 0.66 :`B` 1.0 :`A` 1.0) 0.0))

(fn `OnZombieKilled`
  (params (Zombie :type "/Game/Root/Zombie/AI_Zombie/BP_Zombie Object Reference"))
  ;[1 1 1] Subtract zombie from the array
  (`KismetArrayLibrary.Array_RemoveItem` (`self.Zombies`) Zombie))

(fn `OnZombieSpawned`
  (params (Zombie :type "/Game/Root/Zombie/AI_Zombie/BP_Zombie Object Reference"))
  ;[1 1 1] Add zombie to the array
  (`KismetArrayLibrary.Array_Add` (`self.Zombies`) Zombie)
  (add `/Game/Root/Zombie/AI_Zombie/BP_Zombie.OnKilled` Zombie (`|CreateDelegate` :!event `OnZombieKilled`)))

(fn `UserConstructionScript`)